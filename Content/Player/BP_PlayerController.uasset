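; Player controller that sets up player input and shows a debug readout of the player's location.
; On BeginPlay it adds the default Enhanced Input mapping context and creates the interface widget on the viewport.
; Every tick it writes the first player pawn's position, scaled from centimeters to meters, plus its 3D cell and 2D sector coordinates into the widget's text lines.
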(event EventBeginPlay
  (Input|AddMappingContext (PlayerController|LocalPlayerSubsystems|GetEnhancedInputLocalPlayerSubsystem) "/Game/Input/IMC_Default.IMC_Default" 0 "(bIgnoreAllPressedKeysUntilRelease=True,bForceImmediately=False,bNotifyUserSettings=False)")
  (bind _returnvalue (UserInterface|CreateWidget "/Game/UI/WBP_Interface.WBP_Interface_C" self))
  (UserInterface|Viewport|AddtoViewport _returnvalue 0)
  (Variables|Default|SetInterfaceRef _returnvalue))

(event EventTick
  (params (DeltaSeconds :type Float%20%28single-precision%29))
  (CallFunction|DisplayDebug))

(fn ConstructionScript)

(fn DisplayDebug
  (LocalVariables|SetPlayerLocation (Transformation|GetActorLocation (Game|Player|GetPlayerPawn 0)))
  (Utilities|FlowControl|Sequence
    (:then_0
      (Variables|/Script/UMG.TextBlock|SetText (Variables|/Game/UI/WBP_Interface.WBP_Interface_C|GetTextLine1 (Variables|Default|GetInterfaceRef)) (Utilities|Text|FormatText "Position: {0} {1} {2}" (Utilities|Text|ToText(Float) (.X (Math|Vector|BreakVector (/ (LocalVariables|GetPlayerLocation) 1e+02))) "HalfToEven" false true 1 324 1 1) (Utilities|Text|ToText(Float) (.Y (Math|Vector|BreakVector (/ (LocalVariables|GetPlayerLocation) 1e+02))) "HalfToEven" false true 1 324 1 1) (Utilities|Text|ToText(Float) (.Z (Math|Vector|BreakVector (/ (LocalVariables|GetPlayerLocation) 1e+02))) "HalfToEven" false true 1 324 1 1))))
    (:then_1
      (Variables|/Script/UMG.TextBlock|SetText (Variables|/Game/UI/WBP_Interface.WBP_Interface_C|GetTextLine2 (Variables|Default|GetInterfaceRef)) (Utilities|Text|FormatText "Cell: {0} {1} {2}" (.X (Utilities|Struct|BreakIntVector (Class|VoxelWorld|WorldLocationtoCellCoordinate (LocalVariables|GetPlayerLocation)))) (.Y (Utilities|Struct|BreakIntVector (Class|VoxelWorld|WorldLocationtoCellCoordinate (LocalVariables|GetPlayerLocation)))) (.Z (Utilities|Struct|BreakIntVector (Class|VoxelWorld|WorldLocationtoCellCoordinate (LocalVariables|GetPlayerLocation)))))))
    (:then_2
      (Variables|/Script/UMG.TextBlock|SetText (Variables|/Game/UI/WBP_Interface.WBP_Interface_C|GetTextLine3 (Variables|Default|GetInterfaceRef)) (Utilities|Text|FormatText "Sector {0} {1}" (.X (Utilities|Struct|BreakIntVector2 (Class|VoxelWorld|WorldLocationtoSectorCoordinate (LocalVariables|GetPlayerLocation)))) (.Y (Utilities|Struct|BreakIntVector2 (Class|VoxelWorld|WorldLocationtoSectorCoordinate (LocalVariables|GetPlayerLocation)))))))))